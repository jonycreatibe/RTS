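; Placeable base resource that NPC tasks harvest, tracking quantity in a ResourceInfo struct and a widget progress bar.
; GiveResource deducts a multiplier-scaled yield, updates the bar and returns amount, type, cooldown and whether to find a new resource.
; UpdateQuantityProgressBarVisibility hides the depleted bar and starts a timed respawn that refills it; the destroy path is unwired.
; ShowResourceInfo sends object info to the GameInstance for the info panel.
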(event `self.ReceiveBeginPlay`
  (bind (_resource_info__type _resource_info__quantity _resource_info__quantitypertask _resource_info__initialquantity) (break `/Game/StudentName/Placeables/Resources/S_ResourceInfo` (`self.resource_info_`)))
  (bind _wb_progress_bar_ref_ (`self.wb_progress_bar_ref_`))
  (bind _returnvalue (/ _resource_info__quantity _resource_info__initialquantity))
  ;[1 1 1] Precatching zone.
  (bind _aswb_progress_bar (cast `/Game/StudentName/UI/WB_ProgressBar` (`WidgetComponent.GetUserWidgetObject` (`self.QuantityProgressBar`))))
  (set `self.wb_progress_bar_ref_` _aswb_progress_bar)
  (bind _asbp_game_instance (cast `/Game/StudentName/Framework/BP_GameInstance` (`GameplayStatics.GetGameInstance`)))
  (set `self.game_instance_ref_` _asbp_game_instance)
  ;[1 1 1] Checks progress bar initial visibility.
  (`/Engine/EditorBlueprintResources/StandardMacros.IsValid` _wb_progress_bar_ref_
    (:`Is Valid`
      (`/Game/StudentName/UI/WB_ProgressBar.UpdateElementProgressBar` _wb_progress_bar_ref_ _returnvalue)
      (if (>= _returnvalue 1.0)
        (`SceneComponent.SetVisibility` (`self.QuantityProgressBar`) false true)
        (else
          (`SceneComponent.SetVisibility` (`self.QuantityProgressBar`) true true))))))

(event `RespawnEvent`
  (bind (_resource_info__type _resource_info__quantity _resource_info__quantitypertask _resource_info__initialquantity _resource_info__taskcooldown _resource_info__taskmultiplier _resource_info__respawncooldown) (break `/Game/StudentName/Placeables/Resources/S_ResourceInfo` (`self.resource_info_`)))
  ;[1 1 1] Respawn event (called from "GiveResource" method).
  (`KismetSystemLibrary.K2_SetTimerDelegate` (delegate `RespawnEvent_Action`) _resource_info__respawncooldown))

(event `DestroyEvent`
  ;[1 1 1] Destruction event (called from "GiveResource" method). This couldn't be never called if the resource is destroyed when it's over.
  (`KismetSystemLibrary.K2_SetTimerDelegate` (delegate `DestructionEvent_Action`) 1.0))

(event `DestructionEvent_Action`
  ;[1 1 1] Destruction event (called from "GiveResource" method). This couldn't be never called if the resource is destroyed when it's over.
  (`self.K2_DestroyActor`))

(event `RespawnEvent_Action`
  (bind (_resource_info__type _resource_info__quantity _resource_info__quantitypertask _resource_info__initialquantity) (break `/Game/StudentName/Placeables/Resources/S_ResourceInfo` (`self.resource_info_`)))
  ;[1 1 1] Respawn event (called from "GiveResource" method).
  (bind _structout (setmembers `/Game/StudentName/Placeables/Resources/S_ResourceInfo` :`StructRef` (`self.resource_info_`) :`Quantity` _resource_info__initialquantity :`IsAlive` true))
  (set `self.resource_info_` _structout)
  (`SceneComponent.SetVisibility` (`self.QuantityProgressBar`) false true))

(event `/Game/StudentName/Placeables/Resources/BI_ResourceInfo.ShowResourceInfo`
  ;[1 1 1] Activate the sub panel that show object info.
  (`/Game/StudentName/Framework/BP_GameInstance.UpdateBasicObjectInfo` (`self.game_instance_ref_`) (`self.object_info_`)))

(fn `CheckAlive`
  (returns (`Resource Info  Is Alive` :type Boolean))
  (bind (_resource_info__type _resource_info__quantity _resource_info__quantitypertask _resource_info__initialquantity _resource_info__taskcooldown _resource_info__taskmultiplier _resource_info__respawncooldown _resource_info__shouldrespawn _resource_info__isalive) (break `/Game/StudentName/Placeables/Resources/S_ResourceInfo` (`self.resource_info_`)))
  ;[1 1 1] Method that checks if the resource is alive. This couldn't be never called if the resource is destroyed when it's over.
  (return _resource_info__isalive))

(fn `GetResourceInfo`
  (returns (info :type "/Game/StudentName/Placeables/Resources/S_ResourceInfo Structure"))
  (return (`self.resource_info_`)))

(fn `GetTaskCooldown`
  (returns (cooldown :type "Float (double-precision)"))
  (bind (_resource_info__type _resource_info__quantity _resource_info__quantitypertask _resource_info__initialquantity _resource_info__taskcooldown) (break `/Game/StudentName/Placeables/Resources/S_ResourceInfo` (`self.resource_info_`)))
  (return _resource_info__taskcooldown))

(fn `GiveResource`
  (params (quantity_multiplier_ :type "Float (double-precision)" :default 1.0))
  (returns (quantity :type "Float (double-precision)") (type :type "/Game/StudentName/Placeables/Resources/EResourceType Enum") (cooldown :type "Float (double-precision)") (find_new_resource :type Boolean) (do_it_now :type Boolean))
  (locals (remnant_quantity_ :type "Float (double-precision)" :default 0.0))
  (bind (_resource_info__type _resource_info__quantity _resource_info__quantitypertask _resource_info__initialquantity _resource_info__taskcooldown _resource_info__taskmultiplier _resource_info__respawncooldown _resource_info__shouldrespawn _resource_info__isalive) (break `/Game/StudentName/Placeables/Resources/S_ResourceInfo` (`self.resource_info_`)))
  (bind _returnvalue (/ _resource_info__quantity _resource_info__initialquantity))
  (bind _returnvalue_2 (* quantity_multiplier_ _resource_info__quantitypertask _resource_info__taskmultiplier))
  (bind _returnvalue_3 (- _resource_info__quantity _returnvalue_2))
  ;[1 1 1] This function gives automatically the correct quantity of resources to the NPC once the task has been done.
  (if _resource_info__isalive
    (bind _structout (setmembers `/Game/StudentName/Placeables/Resources/S_ResourceInfo` :`StructRef` (`self.resource_info_`) :`Quantity` _returnvalue_3))
    (set `self.resource_info_` _structout)
    (set `local.remnant_quantity_` (+ _returnvalue_2 _resource_info__quantity))
    (if (<= _returnvalue_3 (- 0.0 _returnvalue_2))
      (`/Game/StudentName/UI/WB_ProgressBar.UpdateElementProgressBar` (`self.wb_progress_bar_ref_`) _returnvalue)
      (bind _structout_2 (setmembers `/Game/StudentName/Placeables/Resources/S_ResourceInfo` :`StructRef` (`self.resource_info_`) :`IsAlive` false))
      (set `self.resource_info_` _structout_2)
      (if _resource_info__shouldrespawn
        (return (`local.remnant_quantity_`) _resource_info__type _resource_info__taskcooldown true false)
        (else
          (return (`local.remnant_quantity_`) _resource_info__type _resource_info__taskcooldown true false)))
      (else
        (`/Game/StudentName/UI/WB_ProgressBar.UpdateElementProgressBar` (`self.wb_progress_bar_ref_`) _returnvalue)
        (`SceneComponent.SetVisibility` (`self.QuantityProgressBar`) true true)
        (return _returnvalue_2 _resource_info__type _resource_info__taskcooldown false false)))
    (else
      (return 0.0 _resource_info__type 0.0 true true))))

(fn `UpdateQuantityProgressBarVisibility`
  (bind (_resource_info__type _resource_info__quantity) (break `/Game/StudentName/Placeables/Resources/S_ResourceInfo` (`self.resource_info_`)))
  (if (<= _resource_info__quantity 0.0)
    (`SceneComponent.SetVisibility` (`self.QuantityProgressBar`) false true)
    (`self.RespawnEvent`)
    (return)
    (else
      (return))))

(fn `UserConstructionScript`)