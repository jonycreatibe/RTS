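; BP_House is a placeable building Blueprint that contributes population to the game.
; When built, it overrides the parent's ExecuteActionWhenBuilt without calling it, passing BuildingPopulation to the game state's UpdatePopulationAndInfo if that reference is valid.
; When destroyed, it calls UpdatePopulationWhenDestroyed, which a TODO flags for designers to adapt.
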(event `self.ReceiveDestroyed`
  ;[1 1 1] TODO designer: adapt this functionality developed in "Event Destroyed" to your game.
  (`self.UpdatePopulationWhenDestroyed`))

(fn `ExecuteActionWhenBuilt`
  (bind _game_state_ref_ (`self.game_state_ref_`))
  ;[1 1 1] Don't call parent functionality.
  (`/Engine/EditorBlueprintResources/StandardMacros.IsValid` _game_state_ref_
    (:`Is Valid`
      (`/Game/StudentName/Framework/BP_GameState.UpdatePopulationAndInfo` _game_state_ref_ (`self.building_population_`))
      (return))
    (:`Is Not Valid`
      (return))))

(fn `UserConstructionScript`
  (`parent.UserConstructionScript`))