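; BP_BasicBuilding is the parent class for placeable buildings, handling construction, selection and worker population.
; On BeginPlay it builds instantly or runs a looping timer feeding a progress bar, then calls ExecuteActionWhenBuilt.
; Built buildings send basic or producer info to the GameInstance UI; worker changes are bounds-checked against GameState population and building capacity.
; Completion, destruction, active-state and worker-multiplier hooks are stubs for child classes to override.
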(event `self.ReceiveBeginPlay`
  ;[1 1 1] Precatching zone.
  (bind _asbp_game_instance (cast `/Game/StudentName/Framework/BP_GameInstance` (`GameplayStatics.GetGameInstance`)))
  (set `self.game_instance_ref_` _asbp_game_instance)
  (bind _aswb_progress_bar (cast `/Game/StudentName/UI/WB_ProgressBar` (`WidgetComponent.GetUserWidgetObject` (`self.ConstructionProgressBar`))))
  (set `self.construction_widget_ref_` _aswb_progress_bar)
  (bind _asbp_game_state (cast `/Game/StudentName/Framework/BP_GameState` (`GameplayStatics.GetGameState`)))
  (set `self.game_state_ref_` _asbp_game_state)
  ;[1 1 1] Comment
  (if (`self.instant_build_`)
    ;;[1 1 1] When the construction of the new building should be instantaneously...
    (`SceneComponent.SetVisibility` (`self.ConstructionProgressBar`) false true)
    (set `self.building_built_` true)
    (`self.ExecuteActionWhenBuilt`)
    (else
      ;;[1 1 1] When we have a little cooldown to finish the new construction:
      (bind _returnvalue (`KismetSystemLibrary.K2_SetTimerDelegate` (delegate `CustomEvent_0`) (`self.time_build_step_`) true))
      (set `self.build_timer_handle_` _returnvalue))))

(event `CustomEvent_0`
  (bind _construction_widget_ref_ (`self.construction_widget_ref_`))
  ;[1 1 1] Comment
  ;;[1 1 1] When we have a little cooldown to finish the new construction:
  (`/Engine/EditorBlueprintResources/StandardMacros.IsValid` _construction_widget_ref_
    (:`Is Valid`
      (bind _output_get (set `self.current_time_build_` (+ (`self.current_time_build_`) (`self.time_build_step_`))))
      (`/Game/StudentName/UI/WB_ProgressBar.UpdateElementProgressBar` _construction_widget_ref_ _output_get)
      (if (>= _output_get (`self.time_to_build_`))
        (`KismetSystemLibrary.K2_ClearAndInvalidateTimerHandle` (`self.build_timer_handle_`))
        (set `self.building_built_` true)
        (`SceneComponent.SetVisibility` (`self.ConstructionProgressBar`) false true)
        (`self.ExecuteActionWhenBuilt`)))))

(event `/Game/StudentName/Placeables/Buildings/BI_BuildingSettings.ChangeBuildingSelectionState`
  (params (is_visible :type Boolean))
  ;[1 1 1] Changes building selection state.
  (`SceneComponent.SetVisibility` (`self.SelectionWidget`) is_visible true))

(event `/Game/StudentName/Placeables/Buildings/BI_BuildingSettings.ShowObjectInfo`
  ;[1 1 1] Activate the sub panel that show object description info.
  (if (`self.building_built_`)
    ;;[1 1 1] TODO designer: remove "producer_building_" boolean if you don't want to differentiate between producer buildings (e.g.: lumbercamp or sawmill) or non producer buildings (e.g.: houses? Town Center? Design dependant).
    (if (`self.producer_building_`)
      (`/Game/StudentName/Framework/BP_GameInstance.UpdateAdvancedObjectInfo` (`self.game_instance_ref_`) (`self.description_info_`) self (`self.building_workers_`) (`self.building_max_workers_`))
      (else
        (`/Game/StudentName/Framework/BP_GameInstance.UpdateBasicObjectInfo` (`self.game_instance_ref_`) (`self.description_info_`))))))

(event `self.ReceiveDestroyed`
  ;[1 1 1] Don't do anything in this point!! Reimplement this event in inherited classes.
  (`KismetSystemLibrary.PrintString` "\"EVENT DESTROYED\" called in \"BP_BasicBuilding\" because of this event doesn't exist in any inherit class (the one related with the building you destroyed)."))

(fn `ChangeActiveState`
  ;[1 1 1] TODO designer: don't do anything in this method in parent class, override it in inherited classes only when needed.
  (return))

(fn `ExecuteActionWhenBuilt`
  ;[1 1 1] Don't do anything in this parent function, develop all the functionality in overrided methods.
  (`KismetSystemLibrary.PrintString` "THIS PARENT METHOD SHOULDN'T BE CALLED, look at \"ExecuteActionWhenBuilt\" method in son classes of \"BP_BasicBuilding\".")
  (return))

(fn `UpdateActivePopulation`
  (params (addition :type Integer) (call_update_population :type Boolean))
  (bind _game_state_ref_ (`self.game_state_ref_`))
  (bind _game_instance_ref_ (`self.game_instance_ref_`))
  (bind _game_state_ref__2 (`self.game_state_ref_`))
  (bind _returnvalue (+ addition (`self.building_workers_`)))
  (bind _returnvalue_2 (+ addition (`self.building_workers_`)))
  (bind _returnvalue_3 (+ addition (`/Game/StudentName/Framework/BP_GameState.active_population_` (`self.game_state_ref_`))))
  (bind _returnvalue_4 (+ (`/Game/StudentName/Framework/BP_GameState.active_population_` _game_state_ref_) addition))
  (`/Engine/EditorBlueprintResources/StandardMacros.IsValid` _game_state_ref_
    (:`Is Valid`
      (if (> addition 0)
        (if (and (<= _returnvalue_4 (`/Game/StudentName/Framework/BP_GameState.population_` _game_state_ref_)) (<= _returnvalue_2 (`self.building_max_workers_`)))
          (set `/Game/StudentName/Framework/BP_GameState.active_population_` _returnvalue_4 _game_state_ref_)
          (set `self.building_workers_` _returnvalue_2)
          (if call_update_population :!label _label
            (`/Engine/EditorBlueprintResources/StandardMacros.IsValid` _game_instance_ref_
              (:`Is Valid`
                (`/Game/StudentName/Framework/BP_GameInstance.UpdatePopulation` _game_instance_ref_ (`/Game/StudentName/Framework/BP_GameState.active_population_` _game_state_ref__2) (`/Game/StudentName/Framework/BP_GameState.population_` _game_state_ref__2))))))
        (elif (and (>= _returnvalue 0) (>= _returnvalue_3 0))
          (set `/Game/StudentName/Framework/BP_GameState.active_population_` _returnvalue_3 _game_state_ref_)
          (set `self.building_workers_` _returnvalue)
          (goto _label))))))

(fn `UpdateInfo`
  (params (mesh :type "StaticMesh Object Reference") (type :type "/Game/StudentName/Placeables/Buildings/EBuildingType Enum" :default "NewEnumerator2") (can_spawn :type Boolean) (data_table_name :type Name) (zone_type :type "/Game/StudentName/Placeables/Zones/EZoneType Enum" :default "NewEnumerator0"))
  (returns (mesh_correct :type Boolean))
  (bind _returnvalue (`StaticMeshComponent.SetStaticMesh` (`self.StaticMesh`) mesh))
  (set `self.type_` type)
  (set `self.zone_type_` zone_type)
  (set `self.dt_prefab_construction_cost_row_` data_table_name)
  (return _returnvalue))

(fn `UpdatePopulationWhenDestroyed`
  (bind _game_state_ref_ (`self.game_state_ref_`))
  (bind _game_instance_ref_ (`self.game_instance_ref_`))
  (bind _game_state_ref__2 (`self.game_state_ref_`))
  (`self.UpdateActivePopulation` (* (`self.building_workers_`) -1))
  (`/Engine/EditorBlueprintResources/StandardMacros.IsValid` _game_state_ref__2
    (:`Is Valid`
      (`/Game/StudentName/Framework/BP_GameState.UpdatePopulation` _game_state_ref__2 (* (`self.building_population_`) -1))
      (`/Game/StudentName/Framework/BP_GameState.CheckIfWorkersExceedsPopulation` _game_state_ref__2)
      (`/Engine/EditorBlueprintResources/StandardMacros.IsValid` _game_instance_ref_
        (:`Is Valid`
          (`/Game/StudentName/Framework/BP_GameInstance.UpdatePopulation` _game_instance_ref_ (`/Game/StudentName/Framework/BP_GameState.active_population_` _game_state_ref_) (`/Game/StudentName/Framework/BP_GameState.population_` _game_state_ref_)))))))

(fn `UpdateWorkerMultiplier`
  ;[1 1 1] TODO designer: don't do anything in this base method.
  (return))

(fn `UserConstructionScript`)