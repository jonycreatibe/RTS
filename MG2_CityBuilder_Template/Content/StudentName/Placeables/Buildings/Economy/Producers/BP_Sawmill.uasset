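; Sawmill economy building that turns wood into money over time, using tech-driven speed and gold yield.
; By default, it spawns a transporter worker at its door whose deliveries start a timed, progress-bar conversion of the delivered amount.
; FastMode skips the transporter, with a looping timer consuming global Wood until empty.
; Toggling active state starts or stops the timer or transporter, and destruction updates population and removes both.
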(event `self.ManualActivationWidget`
  ;[1 1 1] Event called from "ChangeActiveState" method.
  (if (`self.fast_mode_`)
    ;[1 1 1] Fast production mode example of a "Sawmill" building.
    (if (>= (`/Game/StudentName/Framework/BP_GameState.wood_` (`self.game_state_ref_`)) 0.0)
      (`SceneComponent.SetVisibility` (`self.ConstructionProgressBar`) true true)
      (bind _returnvalue (`KismetSystemLibrary.K2_SetTimerDelegate` (delegate `ManualActivationTimer`) 0.032 true))
      (set `self.task_timer_` _returnvalue)
      (`/Game/StudentName/UI/WB_ProgressBar.UpdateElementProgressBar` (`self.construction_widget_ref_`) 0.0)
      (set `self.producing_` true))
    (else
      ;[1 1 1] Transporter mode example of a "Sawmill" building. Default "fast_mode" attribute state is equal to false, so this is the default executed branch.
      (`/Game/StudentName/NPC/BP_NPC.ChangeDeactivatedState` (`self.transporter_ref_`) (not (`self.active_state_`))))))

(event `ManualActivationTimer`
  (bind _game_state_ref_ (`self.game_state_ref_`))
  (bind (_towncenter _house _storage _lumbercamp _sawmill _goldminery _ironminery _sawmillspeed _sawmillgold) (break `/Game/StudentName/UI/TechnologyTree/TechTreeTasks/S_TechCollection` (`/Game/StudentName/Framework/BP_GameState.techs_` (`self.game_state_ref_`))))
  (bind _returnvalue (- (`/Game/StudentName/Framework/BP_GameState.wood_` _game_state_ref_) 1.0))
  ;[1 1 1] Fast production mode example of a "Sawmill" building.
  (bind _output_get (set `self.accum_time_` (+ (`self.accum_time_`) 0.032)))
  (`/Game/StudentName/UI/WB_ProgressBar.UpdateElementProgressBar` (`self.construction_widget_ref_`) (/ _output_get _sawmillspeed))
  (if (>= (`self.accum_time_`) _sawmillspeed)
    (set `self.accum_time_` 0.0)
    (set `/Game/StudentName/Framework/BP_GameState.money_` (+ (`/Game/StudentName/Framework/BP_GameState.money_` _game_state_ref_) (select `bool` (< _returnvalue 0.0) :`false` _sawmillgold :`true` (* (+ 1.0 _returnvalue) _sawmillgold))) _game_state_ref_)
    (bind _output_get_2 (set `/Game/StudentName/Framework/BP_GameState.wood_` _returnvalue _game_state_ref_))
    (if (<= _output_get_2 0.0)
      (set `/Game/StudentName/Framework/BP_GameState.wood_` 0.0 _game_state_ref_)
      (`KismetSystemLibrary.K2_ClearAndInvalidateTimerHandle` (`self.task_timer_`))
      (`SceneComponent.SetVisibility` (`self.ConstructionProgressBar`) false true))
    (`/Game/StudentName/Framework/BP_GameInstance.UpdateResourcesInfo` (`self.game_instance_ref_`))
    (set `self.producing_` false)))

(event `self.ManualDeactivationWidget`
  ;[1 1 1] Event called from "ChangeActiveState" method.
  (if (`self.fast_mode_`)
    (`KismetSystemLibrary.K2_ClearAndInvalidateTimerHandle` (`self.task_timer_`))
    (set `self.accum_time_` 0.0)
    (`SceneComponent.SetVisibility` (`self.ConstructionProgressBar`) false true)
    (set `self.producing_` false)
    (else
      (`/Game/StudentName/NPC/BP_NPC.ChangeDeactivatedState` (`self.transporter_ref_`) (not (`self.active_state_`))))))

(event `self.ManualActivationTransporter`
  (params (quantity :type "Float (single-precision)"))
  ;[1 1 1] Manual activation of the transporter worker.
  (set `self.accum_resource_` quantity)
  (`SceneComponent.SetVisibility` (`self.ConstructionProgressBar`) true true)
  (bind _returnvalue (`KismetSystemLibrary.K2_SetTimerDelegate` (delegate `CustomEvent`) 0.032 true))
  (set `self.task_timer_` _returnvalue)
  (`/Game/StudentName/UI/WB_ProgressBar.UpdateElementProgressBar` (`self.construction_widget_ref_`) 0.0)
  (set `self.producing_` true))

(event `CustomEvent`
  (bind _transporter_ref_ (`self.transporter_ref_`))
  (bind _game_state_ref_ (`self.game_state_ref_`))
  (bind (_towncenter _house _storage _lumbercamp _sawmill _goldminery _ironminery _sawmillspeed _sawmillgold) (break `/Game/StudentName/UI/TechnologyTree/TechTreeTasks/S_TechCollection` (`/Game/StudentName/Framework/BP_GameState.techs_` (`self.game_state_ref_`))))
  ;[1 1 1] Manual activation of the transporter worker.
  (bind _output_get (set `self.accum_time_` (+ (`self.accum_time_`) 0.032)))
  (`/Game/StudentName/UI/WB_ProgressBar.UpdateElementProgressBar` (`self.construction_widget_ref_`) (/ _output_get _sawmillspeed))
  (if (>= (`self.accum_time_`) _sawmillspeed)
    (set `self.accum_time_` 0.0)
    (set `/Game/StudentName/Framework/BP_GameState.money_` (+ (`/Game/StudentName/Framework/BP_GameState.money_` _game_state_ref_) (* (`self.accum_resource_`) _sawmillgold)) _game_state_ref_)
    (set `self.accum_resource_` 0.0)
    (`KismetSystemLibrary.K2_ClearAndInvalidateTimerHandle` (`self.task_timer_`))
    (`SceneComponent.SetVisibility` (`self.ConstructionProgressBar`) false true)
    (set `self.producing_` false)
    (`/Game/StudentName/Framework/BP_GameInstance.UpdateResourcesInfo` (`self.game_instance_ref_`))
    (if (`/Game/StudentName/NPC/Transporter/BP_Transporter.waiting_to_release_resources_` _transporter_ref_)
      (`/Game/StudentName/NPC/Transporter/BP_Transporter.SetResourceInBuildingMethod` _transporter_ref_))))

(event `self.ReceiveDestroyed`
  (bind _task_timer_ (`self.task_timer_`))
  (bind _transporter_ref_ (`self.transporter_ref_`))
  ;[1 1 1] TODO designer: adapt this functionality developed in "Event Destroyed" to your game.
  (`self.UpdatePopulationWhenDestroyed`)
  (if (`KismetSystemLibrary.K2_IsTimerActiveHandle` _task_timer_)
    (`KismetSystemLibrary.K2_ClearAndInvalidateTimerHandle` _task_timer_))
  (`/Engine/EditorBlueprintResources/StandardMacros.IsValid` _transporter_ref_
    (:`Is Valid`
      (`self.K2_DestroyActor` _transporter_ref_))))

(fn `ChangeActiveState`
  (bind _output_get (set `self.active_state_` (not (`self.active_state_`))))
  (if _output_get
    (`self.ManualActivationWidget`)
    (return)
    (else
      (`self.ManualDeactivationWidget`)
      (return))))

(fn `ExecuteActionWhenBuilt`
  (`/Game/StudentName/Framework/BP_GameState.UpdatePopulationAndInfo` (`self.game_state_ref_`) (`self.building_population_`))
  (if (not (`self.fast_mode_`))
    (bind _returnvalue (`|SpawnActorFromClass` "/Game/StudentName/NPC/Transporter/BP_Transporter.BP_Transporter_C" (`SceneComponent.K2_GetComponentToWorld` (`self.DoorPoint`)) "AdjustIfPossibleButAlwaysSpawn" "OverrideRootScale" null null))
    (bind _output_get (set `self.transporter_ref_` _returnvalue))
    (`/Game/StudentName/NPC/Transporter/BP_Transporter.BasicSetup` _output_get "NewEnumerator0" self)
    (`/Game/StudentName/NPC/BP_NPC.ChangeDeactivatedState` (`self.transporter_ref_`) (not (`self.active_state_`)))
    (`/Game/StudentName/NPC/BP_NPC.UpdateNPCMultiplier` (`self.transporter_ref_`) (/ (`KismetMathLibrary.Conv_IntToDouble` (`self.building_workers_`)) (`KismetMathLibrary.Conv_IntToDouble` (`self.building_max_workers_`)))))
  (return))

(fn `UserConstructionScript`
  (`parent.UserConstructionScript`))