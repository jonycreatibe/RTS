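; BP_ProducerBase is a base economy building that scales production logistics with its assigned worker count.
; UpdateWorkerMultiplier sets ActiveState from whether any workers are present and mirrors it to the referenced transporter's deactivated state.
; It always passes the worker count to the transporter, adding the current-to-maximum worker ratio as an NPC multiplier when staffed.
; The parent implementation is left unconnected, and the event graph and construction script are empty.
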(fn `UpdateWorkerMultiplier`
  ;[1 1 1] This method updates worker multiplier when adding or substracting new workers.
  (if (== (`self.building_workers_`) 0)
    (bind _output_get (set `self.active_state_` false))
    (`/Game/StudentName/NPC/BP_NPC.ChangeDeactivatedState` (`self.transporter_ref_`) (not _output_get))
    (`/Game/StudentName/NPC/BP_NPC.UpdateNumberWorkers` (`self.transporter_ref_`) (`self.building_workers_`))
    (return)
    (else
      (bind _output_get_2 (set `self.active_state_` true))
      (`/Game/StudentName/NPC/BP_NPC.ChangeDeactivatedState` (`self.transporter_ref_`) (not _output_get_2))
      (`/Game/StudentName/NPC/BP_NPC.UpdateNPCMultiplier` (`self.transporter_ref_`) (/ (`KismetMathLibrary.Conv_IntToDouble` (`self.building_workers_`)) (`KismetMathLibrary.Conv_IntToDouble` (`self.building_max_workers_`))))
      (`/Game/StudentName/NPC/BP_NPC.UpdateNumberWorkers` (`self.transporter_ref_`) (`self.building_workers_`))
      (return))))

(fn `UserConstructionScript`)