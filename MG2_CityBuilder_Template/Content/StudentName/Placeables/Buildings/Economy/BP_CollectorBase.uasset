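; BP_CollectorBase is an economy building base that runs resource collection through one spawned BP_Worker.
; When built, it spawns the worker at its door, seeds its AI Blackboard, maps building type to resource type and updates population.
; Staffing sets the worker's multiplier as a ratio of maximum, while zero staff or manual toggling deactivates it.
; Destroying the building updates population and destroys the worker.
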(event `self.ReceiveDestroyed`
  (bind _worker_ref_ (`self.worker_ref_`))
  ;[1 1 1] TODO designer: adapt this functionality developed in "Event Destroyed" to your game.
  (`self.UpdatePopulationWhenDestroyed`)
  (`/Engine/EditorBlueprintResources/StandardMacros.IsValid` _worker_ref_
    (:`Is Valid`
      (`self.K2_DestroyActor` _worker_ref_))))

(event `/Game/StudentName/Placeables/Buildings/BI_BuildingSettings.ManualActivationWidget`
  ;[1 1 1] Event called from "ChangeActiveState" method.
  (`/Game/StudentName/NPC/BP_NPC.ChangeDeactivatedState` (`self.worker_ref_`) (not (`self.active_state_`))))

(event `/Game/StudentName/Placeables/Buildings/BI_BuildingSettings.ManualDeactivationWidget`
  ;[1 1 1] Event called from "ChangeActiveState" method.
  (`/Game/StudentName/NPC/BP_NPC.ChangeDeactivatedState` (`self.worker_ref_`) (not (`self.active_state_`))))

(fn `ChangeActiveState`
  (bind _output_get (set `self.active_state_` (not (`self.active_state_`))))
  (if _output_get
    (`/Game/StudentName/Placeables/Buildings/BI_BuildingSettings.ManualActivationWidget`)
    (return)
    (else
      (`/Game/StudentName/Placeables/Buildings/BI_BuildingSettings.ManualDeactivationWidget`)
      (return))))

(fn `ExecuteActionWhenBuilt`
  ;[1 1 1] TODO designer: this is only an example about how to develop the task executed in some building.
  (bind _returnvalue (`|SpawnActorFromClass` "/Game/StudentName/NPC/Worker/BP_Worker.BP_Worker_C" (`SceneComponent.K2_GetComponentToWorld` (`self.DoorPoint`)) "AlwaysSpawn" "OverrideRootScale" null null))
  (bind _output_get (set `self.worker_ref_` _returnvalue))
  (bind _output_get_2 (set `/Game/StudentName/NPC/BP_NPC.owner_building_ref_` self _output_get))
  (bind _returnvalue_2 (`AIBlueprintHelperLibrary.GetBlackboard` _output_get))
  (`BlackboardComponent.SetValueAsObject` _returnvalue_2 (`/Game/StudentName/NPC/BP_NPC.original_building_ref_key_` _output_get) _output_get_2)
  (`BlackboardComponent.SetValueAsBool` _returnvalue_2 (`/Game/StudentName/NPC/BP_NPC.deactivated_key_` _output_get) (not (`self.active_state_`)))
  (`BlackboardComponent.SetValueAsVector` _returnvalue_2 (`/Game/StudentName/NPC/BP_NPC.original_building_door_point_key_` _output_get) (`SceneComponent.K2_GetComponentLocation` (`self.DoorPoint`)))
  (set `/Game/StudentName/NPC/BP_NPC.resource_type_` (select `/Game/StudentName/Placeables/Buildings/EBuildingType` (`self.type_`) :`NewEnumerator2` "NewEnumerator0" :`NewEnumerator6` "NewEnumerator0" :`NewEnumerator0` "NewEnumerator0" :`NewEnumerator7` "NewEnumerator0" :`NewEnumerator1` "NewEnumerator0" :`NewEnumerator3` "NewEnumerator0" :`NewEnumerator5` "NewEnumerator2" :`NewEnumerator4` "NewEnumerator1" :!type "/Game/StudentName/Placeables/Resources/EResourceType Enum") _output_get)
  (`/Game/StudentName/NPC/BP_NPC.UpdateNPCMultiplier` _output_get (/ (`KismetMathLibrary.Conv_IntToDouble` (`self.building_workers_`)) (`KismetMathLibrary.Conv_IntToDouble` (`self.building_max_workers_`))))
  (`/Game/StudentName/Framework/BP_GameState.UpdatePopulationAndInfo` (`self.game_state_ref_`) (`self.building_population_`))
  (return))

(fn `UpdateWorkerMultiplier`
  (if (== (`self.building_workers_`) 0)
    (bind _output_get (set `self.active_state_` false))
    (`/Game/StudentName/NPC/BP_NPC.ChangeDeactivatedState` (`self.worker_ref_`) (not _output_get))
    (`/Game/StudentName/NPC/BP_NPC.UpdateNumberWorkers` (`self.worker_ref_`) (`self.building_workers_`))
    (return)
    (else
      (bind _output_get_2 (set `self.active_state_` true))
      (`/Game/StudentName/NPC/BP_NPC.ChangeDeactivatedState` (`self.worker_ref_`) (not _output_get_2))
      (`/Game/StudentName/NPC/BP_NPC.UpdateNPCMultiplier` (`self.worker_ref_`) (/ (`KismetMathLibrary.Conv_IntToDouble` (`self.building_workers_`)) (`KismetMathLibrary.Conv_IntToDouble` (`self.building_max_workers_`))))
      (`/Game/StudentName/NPC/BP_NPC.UpdateNumberWorkers` (`self.worker_ref_`) (`self.building_workers_`))
      (return))))

(fn `UserConstructionScript`
  (`parent.UserConstructionScript`))