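; Town Center building, a unique storageable placeable that serves as an example of handling one-of-a-kind buildings.
; BeginPlay sets its flag in the GameState's unique-building state and tells the GameInstance to switch that type's visibility to Hidden.
; Destroyed clears the flag, restores visibility and updates population.
; ExecuteActionWhenBuilt passes the building's population to the GameState without calling the parent version.
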(event `self.ReceiveBeginPlay`
  (bind _game_state_ref_ (`self.game_state_ref_`))
  ;[1 1 1] TODO designer: this is only an example about how to work with an unique building in the "Begin Play" event.
  (`parent.ReceiveBeginPlay`)
  (bind _structout (setmembers `/Game/StudentName/Placeables/Buildings/S_UniqueBuilding` :`StructRef` (`/Game/StudentName/Framework/BP_GameState.unique_buildings_state_` _game_state_ref_) :`TownCenter` true))
  (set `/Game/StudentName/Framework/BP_GameState.unique_buildings_state_` _structout _game_state_ref_)
  (`/Game/StudentName/Framework/BP_GameInstance.UpdateUniqueBuildingState` (`self.game_instance_ref_`) "NewEnumerator6" "Hidden"))

(event `self.ReceiveDestroyed`
  (bind _game_state_ref_ (`self.game_state_ref_`))
  ;[1 1 1] TODO designer: this is only an example about how to work with an unique building in the "Destroyed" event.
  (`/Engine/EditorBlueprintResources/StandardMacros.IsValid` _game_state_ref_
    (:`Is Valid`
      (bind _structout (setmembers `/Game/StudentName/Placeables/Buildings/S_UniqueBuilding` :`StructRef` (`/Game/StudentName/Framework/BP_GameState.unique_buildings_state_` _game_state_ref_) :`TownCenter` false))
      (set `/Game/StudentName/Framework/BP_GameState.unique_buildings_state_` _structout _game_state_ref_)
      (`/Game/StudentName/Framework/BP_GameInstance.UpdateUniqueBuildingState` (`self.game_instance_ref_`) "NewEnumerator6" "Visible")
      (`self.UpdatePopulationWhenDestroyed`))))

(fn `ExecuteActionWhenBuilt`
  (bind _game_state_ref_ (`self.game_state_ref_`))
  ;[1 1 1] TODO designer: some stuff.
  (`/Engine/EditorBlueprintResources/StandardMacros.IsValid` _game_state_ref_
    (:`Is Valid`
      (`/Game/StudentName/Framework/BP_GameState.UpdatePopulationAndInfo` _game_state_ref_ (`self.building_population_`))
      (return))
    (:`Is Not Valid`
      (return))))

(fn `UserConstructionScript`
  (`parent.UserConstructionScript`))