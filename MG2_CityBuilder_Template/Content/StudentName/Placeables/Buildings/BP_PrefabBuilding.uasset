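; Placement prefab for a building that tracks whether it can be spawned at its current spot.
; It counts overlaps with tagged buildings and resources to toggle CanSpawn.
; In grid world mode, its Box compares overlapped BI_Zone types with its own and reports zone validity to BP_Pawn.
; It extends a parent building class, forcing InstantBuild, adding CanSpawn to UpdateInfo and suppressing the built action.
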(event `self.ReceiveBeginPlay`
  ;[1 1 1] Basic events.
  (set `self.instant_build_` true)
  (bind _returnvalue (`GameplayStatics.GetActorOfClass` "/Game/StudentName/Placeables/BP_GridWorld.BP_GridWorld_C"))
  (set `self.world_ref_` _returnvalue)
  (bind _asbp_pawn (cast `/Game/StudentName/Framework/BP_Pawn` (`GameplayStatics.GetPlayerPawn` 0)))
  (set `self.pawn_ref_` _asbp_pawn)
  (`parent.ReceiveBeginPlay`))

(event `self.ReceiveTick`
  (params (DeltaSeconds :type "Float (single-precision)"))
  ;[1 1 1] Basic events.
  (`parent.ReceiveTick` DeltaSeconds))

(event `self.ReceiveActorBeginOverlap`
  (params (OtherActor :type "Actor Object Reference"))
  ;[1 1 1] Checks if this prefab overlaps with another building or resource item.
  (if (or (`self.ActorHasTag` OtherActor "BasicBuilding") (`self.ActorHasTag` OtherActor "BasicResource"))
    (set `self.can_spawn_` false)
    (`/Engine/EditorBlueprintResources/StandardMacros.IncrementInt` (`self.overlap_counter_`))))

(event `self.ReceiveActorEndOverlap`
  (params (OtherActor :type "Actor Object Reference"))
  ;[1 1 1] Checks if this prefab loses its collision with another building or resource item.
  (if (or (`self.ActorHasTag` OtherActor "BasicBuilding") (`self.ActorHasTag` OtherActor "BasicResource"))
    (bind _result (`/Engine/EditorBlueprintResources/StandardMacros.DecrementInt` (`self.overlap_counter_`))
      (:`  `
        (if (== _result 0)
          (set `self.can_spawn_` true))))))

(event `self.Box.OnComponentBeginOverlap`
  (params (OverlappedComponent :type "PrimitiveComponent Object Reference") (OtherActor :type "Actor Object Reference") (OtherComp :type "PrimitiveComponent Object Reference") (OtherBodyIndex :type Integer) (bFromSweep :type Boolean) (SweepResult :type "HitResult Structure (by ref)"))
  (bind _pawn_ref_ (`self.pawn_ref_`))
  ;[1 1 1] Spawning in grid world mode.
  (if (and (`KismetSystemLibrary.DoesImplementInterface` OtherActor "/Game/StudentName/Placeables/Zones/BI_Zone.BI_Zone_C") (`|EnumEquality` (`/Game/StudentName/Placeables/BP_GridWorld.world_type_` (`self.world_ref_`)) "NewEnumerator1"))
    (bind _zone (message `/Game/StudentName/Placeables/Zones/BI_Zone.GetZoneType` OtherActor))
    (set `/Game/StudentName/Framework/BP_Pawn.last_zone_type_` _zone (`self.pawn_ref_`))
    (if (or (`|EnumEquality` _zone "NewEnumerator0") (`|EnumEquality` _zone (`self.zone_type_`)) (`|EnumEquality` (`self.zone_type_`) "NewEnumerator0"))
      (set `/Game/StudentName/Framework/BP_Pawn.can_spawn_in_zone_` true _pawn_ref_)
      (else
        (set `/Game/StudentName/Framework/BP_Pawn.can_spawn_in_zone_` false _pawn_ref_)))))

(event `self.Box.OnComponentEndOverlap`
  (params (OverlappedComponent :type "PrimitiveComponent Object Reference") (OtherActor :type "Actor Object Reference") (OtherComp :type "PrimitiveComponent Object Reference") (OtherBodyIndex :type Integer))
  ;[1 1 1] Spawning in grid world mode.
  (if (and (`KismetSystemLibrary.DoesImplementInterface` OtherActor "/Game/StudentName/Placeables/Zones/BI_Zone.BI_Zone_C") (`|EnumEquality` (`/Game/StudentName/Placeables/BP_GridWorld.world_type_` (`self.world_ref_`)) "NewEnumerator1"))
    (bind _zone (message `/Game/StudentName/Placeables/Zones/BI_Zone.GetZoneType` OtherActor))
    (if (and (`|EnumInequality` _zone "NewEnumerator0") (`|EnumEquality` _zone (`self.zone_type_`)))
      (set `/Game/StudentName/Framework/BP_Pawn.can_spawn_in_zone_` false (`self.pawn_ref_`)))))

(fn `ExecuteActionWhenBuilt`
  ;[1 1 1] Don't do anything in this method.
  (return))

(fn `UpdateInfo`
  (params (mesh :type "StaticMesh Object Reference") (type :type "/Game/StudentName/Placeables/Buildings/EBuildingType Enum" :default "NewEnumerator2") (can_spawn :type Boolean) (data_table_name :type Name) (zone_type :type "/Game/StudentName/Placeables/Zones/EZoneType Enum" :default "NewEnumerator0"))
  (returns (mesh_correct :type Boolean))
  (bind _mesh_correct (`parent.UpdateInfo` mesh type false data_table_name zone_type))
  (set `self.can_spawn_` can_spawn)
  (return _mesh_correct))

(fn `UserConstructionScript`
  (`parent.UserConstructionScript`))