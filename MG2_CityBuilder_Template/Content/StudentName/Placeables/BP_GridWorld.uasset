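; Placeable grid world actor that defines the map area from two beacon actors, as a free, squared-grid or optionally circular map.
; Its construction script scales the actor so the plane's size matches the beacon separation, then computes cell sizes for squared grids.
; Grid counts and the circular flag drive the plane's material parameters.
; Getters expose X/Y bounds from the beacons, with circular bounds using Beacon1's X and its negation.
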(event `self.ReceiveBeginPlay`)

(fn `GetMaxMapSizeCircular`
  (returns (output :type "Float (double-precision)"))
  (bind _beacon_1_ (`self.beacon_1_`))
  (bind _returnvalue_x (`KismetMathLibrary.BreakVector` (`self.K2_GetActorLocation` _beacon_1_)))
  ;[1 1 1] Takes 'X' axis value of "beacon_1" as maximum value.
  (return (`KismetMathLibrary.SelectFloat` (* _returnvalue_x -1.0) 0.0 (`KismetSystemLibrary.IsValid` _beacon_1_))))

(fn `GetMaxMapSizeX`
  (returns (output :type "Float (double-precision)"))
  (bind _beacon_2_ (`self.beacon_2_`))
  (bind _returnvalue_x (`KismetMathLibrary.BreakVector` (`self.K2_GetActorLocation` _beacon_2_)))
  ;[1 1 1] Gets "beacon_2" position in the 'X' axis (maximum 'X').
  (return (`KismetMathLibrary.SelectFloat` _returnvalue_x 0.0 (`KismetSystemLibrary.IsValid` _beacon_2_))))

(fn `GetMaxMapSizeY`
  (returns (output :type "Float (double-precision)"))
  (bind _beacon_2_ (`self.beacon_2_`))
  (bind (_returnvalue_x _returnvalue_y) (`KismetMathLibrary.BreakVector` (`self.K2_GetActorLocation` _beacon_2_)))
  ;[1 1 1] Gets "beacon_2" position in the 'Y' axis (maximum 'Y').
  (return (`KismetMathLibrary.SelectFloat` _returnvalue_y 0.0 (`KismetSystemLibrary.IsValid` _beacon_2_))))

(fn `GetMinMapSizeCircular`
  (returns (output :type "Float (double-precision)"))
  (bind _beacon_1_ (`self.beacon_1_`))
  (bind _returnvalue_x (`KismetMathLibrary.BreakVector` (`self.K2_GetActorLocation` _beacon_1_)))
  ;[1 1 1] Takes 'X' axis value of "beacon_2" as minimum value.
  (return (`KismetMathLibrary.SelectFloat` _returnvalue_x 0.0 (`KismetSystemLibrary.IsValid` _beacon_1_))))

(fn `GetMinMapSizeX`
  (returns (output :type "Float (double-precision)"))
  (bind _beacon_1_ (`self.beacon_1_`))
  (bind _returnvalue_x (`KismetMathLibrary.BreakVector` (`self.K2_GetActorLocation` _beacon_1_)))
  ;[1 1 1] Gets "beacon_1" position in the 'X' axis (minimum 'X').
  (return (`KismetMathLibrary.SelectFloat` _returnvalue_x 0.0 (`KismetSystemLibrary.IsValid` _beacon_1_))))

(fn `GetMinMapSizeY`
  (returns (output :type "Float (double-precision)"))
  (bind _beacon_1_ (`self.beacon_1_`))
  (bind (_returnvalue_x _returnvalue_y) (`KismetMathLibrary.BreakVector` (`self.K2_GetActorLocation` _beacon_1_)))
  ;[1 1 1] Gets "beacon_1" position in the 'Y' axis (minimum 'Y').
  (return (`KismetMathLibrary.SelectFloat` _returnvalue_y 0.0 (`KismetSystemLibrary.IsValid` _beacon_1_))))

(fn `UserConstructionScript`
  (bind (_min _max) (`StaticMeshComponent.GetLocalBounds` (`self.Plane`)))
  (`/Engine/EditorBlueprintResources/StandardMacros.IsValid` (`self.beacon_2_`)
    (:`Is Valid`
      (`/Engine/EditorBlueprintResources/StandardMacros.IsValid` (`self.beacon_1_`)
        (:`Is Valid`
          (`self.SetActorScale3D` (1.0 1.0 1.0))
          (`self.SetActorScale3D` (`KismetMathLibrary.MakeVector` (/ (.x (- (`self.K2_GetActorLocation` (`self.beacon_2_`)) (`self.K2_GetActorLocation` (`self.beacon_1_`)))) (.x (- _max _min))) (/ (.y (- (`self.K2_GetActorLocation` (`self.beacon_2_`)) (`self.K2_GetActorLocation` (`self.beacon_1_`)))) (.y (- _max _min))) 1.0))
          ;[1 1 1] TODO designer: improve this point if you add more grid types (e.g. hexagonal grid).
          (switch `/Game/StudentName/Placeables/EWorldType` (`self.world_type_`)
            (:`NewEnumerator0`
              (`MeshComponent.SetScalarParameterValueOnMaterials` (`self.Plane`) "NumberCols" 1.0)
              (`MeshComponent.SetScalarParameterValueOnMaterials` (`self.Plane`) "NumberRows" 1.0))
            (:`NewEnumerator1`
              (`MeshComponent.SetScalarParameterValueOnMaterials` (`self.Plane`) "NumberCols" (`self.n_rows_`))
              (`MeshComponent.SetScalarParameterValueOnMaterials` (`self.Plane`) "NumberRows" (`self.n_cols_`))
              (set `self.col_size_` (/ (.x (- (`self.K2_GetActorLocation` (`self.beacon_2_`)) (`self.K2_GetActorLocation` (`self.beacon_1_`)))) (`self.n_cols_`)))
              (set `self.row_size_` (/ (.y (- (`self.K2_GetActorLocation` (`self.beacon_2_`)) (`self.K2_GetActorLocation` (`self.beacon_1_`)))) (`self.n_rows_`)))))
          ;[1 1 1] Is our map a circular map?
          (if (`self.circular_map_`)
            (`MeshComponent.SetScalarParameterValueOnMaterials` (`self.Plane`) "Circular" 1.0)
            (else
              (`MeshComponent.SetScalarParameterValueOnMaterials` (`self.Plane`) "Circular" 0.0))))))))