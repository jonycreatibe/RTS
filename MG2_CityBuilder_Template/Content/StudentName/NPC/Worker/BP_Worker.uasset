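; BP_Worker is an NPC worker that carries a typed resource quantity for its behavior tree, BT_Worker.
; On BeginPlay it caches a BP_GameState reference.
; StoreResource adds the carried amount to the game state through UpdateResource and zeroes it, while DestroyResource discards it when a building is deactivated.
; GetResourceTypeTask exposes the worker's resource type.
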(event `self.ReceiveBeginPlay`
  (bind _asbp_game_state (cast `/Game/StudentName/Framework/BP_GameState` (`GameplayStatics.GetGameState`)))
  (set `self.game_state_ref_` _asbp_game_state))

(event `/Game/StudentName/NPC/Worker/BI_Worker.StoreResource`
  ;[1 1 1] Called from "BT_Worker" behavior tree when storing resources on its respective building.
  (`/Game/StudentName/Framework/BP_GameState.UpdateResource` (`self.game_state_ref_`) (`self.resource_type_`) (`self.resource_quantity_`))
  (set `self.resource_quantity_` 0.0))

(event `/Game/StudentName/NPC/Worker/BI_Worker.DestroyResource`
  ;[1 1 1] Called from "BT_Worker" behavior tree when deactivating the building.
  (set `self.resource_quantity_` 0.0))

(fn `GetResourceTypeTask`
  (returns (type :type "/Game/StudentName/Placeables/Resources/EResourceType Enum"))
  (return (`self.resource_type_`)))

(fn `UserConstructionScript`)