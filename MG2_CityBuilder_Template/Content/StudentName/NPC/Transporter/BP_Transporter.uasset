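; Transporter NPC that carries a quantity of one resource type for an owning building, driven by the BT_Transporter behavior tree.
; BasicSetup stores the type and owner, then writes the building and its door point to the Blackboard.
; State functions mirror waiting and resource-existence flags to the Blackboard.
; Drop-off clears the load and either returns the amount or passes it to the owner's ManualActivationTransporter; deactivation zeroes it.
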(event `/Game/StudentName/NPC/Transporter/BI_Transporter.SetWaitState`
  (params (state :type Boolean))
  ;[1 1 1] Called from "BT_Transporter" behavior tree when storing resources on its respective building.
  (bind _output_get (set `self.waiting_to_release_resources_` state))
  (`BlackboardComponent.SetValueAsBool` (`AIBlueprintHelperLibrary.GetBlackboard` null) (`self.waiting_to_release_resources_key_`) _output_get))

(event `/Game/StudentName/NPC/Transporter/BI_Transporter.DestroyResource`
  ;[1 1 1] Called from "BT_Transporter" behavior tree when deactivating the building.
  (set `self.resource_quantity_` 0.0))

(fn `BasicSetup`
  (params (type :type "/Game/StudentName/Placeables/Resources/EResourceType Enum" :default "NewEnumerator0") (building_owner_ :type "/Game/StudentName/Placeables/Buildings/BP_BasicBuilding Object Reference"))
  (bind _returnvalue (`AIBlueprintHelperLibrary.GetBlackboard` null))
  ;[1 1 1] Sets resource type, original building ref and behavior tree blackboard information.
  (set `self.resource_type_` type)
  (bind _output_get (set `self.owner_building_ref_` building_owner_))
  (`BlackboardComponent.SetValueAsObject` _returnvalue (`self.original_building_ref_key_`) _output_get)
  (`BlackboardComponent.SetValueAsVector` _returnvalue (`self.original_building_door_point_key_`) (`SceneComponent.K2_GetComponentLocation` (`/Game/StudentName/Placeables/Buildings/BP_BasicBuilding.DoorPoint` _output_get))))

(fn `CheckIfResourceExist`
  (params (state :type Boolean))
  (`BlackboardComponent.SetValueAsBool` (`AIBlueprintHelperLibrary.GetBlackboard` null) (`self.exist_resource_key_`) state))

(fn `GetOwnerBuilding`
  (returns (owner_building :type "/Game/StudentName/Placeables/Buildings/BP_BasicBuilding Object Reference"))
  (return (`self.owner_building_ref_`)))

(fn `GetResourceTypeTask`
  (returns (type :type "/Game/StudentName/Placeables/Resources/EResourceType Enum"))
  (return (`self.resource_type_`)))

(fn `SetResourceInBuilding`
  (returns (quantity :type "Float (double-precision)"))
  (locals (previous_resource_quantity :type "Float (double-precision)"))
  (set `local.previous_resource_quantity` (`self.resource_quantity_`))
  (`BlackboardComponent.SetValueAsBool` (`AIBlueprintHelperLibrary.GetBlackboard` null) (`self.has_resource_key_`) false)
  (bind _output_get (set `self.waiting_to_release_resources_` false))
  (`BlackboardComponent.SetValueAsBool` (`AIBlueprintHelperLibrary.GetBlackboard` null) (`self.waiting_to_release_resources_key_`) _output_get)
  (set `self.resource_quantity_` 0.0)
  (return (`local.previous_resource_quantity`)))

(fn `SetResourceInBuildingMethod`
  (locals (previous_resource_quantity_ :type "Float (double-precision)" :default 0.0))
  (set `local.previous_resource_quantity_` (`self.resource_quantity_`))
  (`BlackboardComponent.SetValueAsBool` (`AIBlueprintHelperLibrary.GetBlackboard` null) (`self.has_resource_key_`) false)
  (bind _output_get (set `self.waiting_to_release_resources_` false))
  (`BlackboardComponent.SetValueAsBool` (`AIBlueprintHelperLibrary.GetBlackboard` null) (`self.waiting_to_release_resources_key_`) _output_get)
  (set `self.resource_quantity_` 0.0)
  (`/Game/StudentName/Placeables/Buildings/BP_BasicBuilding.ManualActivationTransporter` (`self.owner_building_ref_`) (`local.previous_resource_quantity_`))
  (return))

(fn `UserConstructionScript`)