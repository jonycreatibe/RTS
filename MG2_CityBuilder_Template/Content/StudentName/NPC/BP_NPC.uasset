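; BP_NPC is an NPC with a citizens widget, a resource multiplier and a deactivation state.
; On BeginPlay it caches the WB_Citizens instance from its widget component.
; UpdateNumberWorkers passes worker counts to that widget, re-fetching the reference if it is invalid.
; Other functions write the deactivated flag to the AI Blackboard and store a new resource multiplier.
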(event `self.ReceiveBeginPlay`
  ;[1 1 1] Precatching zone.
  (bind _aswb_citizens (cast `/Game/StudentName/UI/WidgetComponent/WB_Citizens` (`WidgetComponent.GetUserWidgetObject` (`self.Widget`))))
  (set `self.wb_citizens_ref_` _aswb_citizens))

(event `self.ReceiveTick`
  (params (DeltaSeconds :type "Float (single-precision)")))

(fn `ChangeDeactivatedState`
  (params (state :type Boolean))
  (`BlackboardComponent.SetValueAsBool` (`AIBlueprintHelperLibrary.GetBlackboard` null) (`self.deactivated_key_`) state))

(fn `UpdateNPCMultiplier`
  (params (new_resource_multiplier :type "Float (double-precision)"))
  (set `self.resource_multiplier_` new_resource_multiplier)
  (return))

(fn `UpdateNumberWorkers`
  (params (workers :type Integer))
  (`/Engine/EditorBlueprintResources/StandardMacros.IsValid` (`self.wb_citizens_ref_`)
    (:`Is Valid`
      (`/Game/StudentName/UI/WidgetComponent/WB_Citizens.UpdateWorkersTxt` (`self.wb_citizens_ref_`) workers))
    (:`Is Not Valid`
      (bind _aswb_citizens (cast `/Game/StudentName/UI/WidgetComponent/WB_Citizens` (`WidgetComponent.GetUserWidgetObject` (`self.Widget`))))
      (bind _output_get (set `self.wb_citizens_ref_` _aswb_citizens))
      (`/Game/StudentName/UI/WidgetComponent/WB_Citizens.UpdateWorkersTxt` _output_get workers))))

(fn `UserConstructionScript`)