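; Player controller for a building game that routes player input to BP_Pawn and BP_HUD.
; BeginPlay caches both references, runs the "show Collision" console command and sets Game-and-UI input with the mouse locked.
; Movement, camera, zoom and building inputs go to the pawn, with CanSpawnPrefab switching spawn/select and clear/show-info.
; The tech tree input toggles the HUD's tree, while pause does nothing yet.
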(event `self.ReceiveBeginPlay`
  ;[1 1 1] Precatching nodes in "BeginPlay" event.
  (bind _asbp_pawn (cast `/Game/StudentName/Framework/BP_Pawn` (`GameplayStatics.GetPlayerPawn` 0))
    (:`then`
      (set `self.bp_player_ref_` _asbp_pawn)
      (bind _asbp_hud (cast `/Game/StudentName/Framework/BP_HUD` (`self.GetHUD`))
        (:`then`
          (set `self.bp_hud_ref_` _asbp_hud)
          (`KismetSystemLibrary.ExecuteConsoleCommand` "show Collision" self)
          ;[1 1 1] This is important to avoid problems while playing with input "A", "W", "S", "D" and mouse movement with borders.
          (`WidgetBlueprintLibrary.SetInputMode_GameAndUIEx` self null "LockAlways"))
        (:`CastFailed`
          (`KismetSystemLibrary.PrintString` "Cast to \"BP_HUD\" failed in \"BeginPlay\" event in the \"BP_PlayerController\"."))))
    (:`CastFailed`
      (`KismetSystemLibrary.PrintString` "Cast to \"BP_Pawn\" failed in \"BeginPlay\" event in the \"BP_PlayerController\"."))))

(event `InputAction|PauseAction` :consume false :paused true
  (params (Key :type "Key Structure"))
  ;[1 1 1] Game inputs to Player and HUD.
  (:`Pressed`
    (`/Engine/EditorBlueprintResources/StandardMacros.IsValid` (`self.bp_hud_ref_`))))

(event `InputAction|SpawnAction` :consume false
  (params (Key :type "Key Structure"))
  (bind _bp_player_ref_ (`self.bp_player_ref_`))
  ;[1 1 1] Game inputs to Player and HUD.
  (:`Pressed`
    (`/Engine/EditorBlueprintResources/StandardMacros.IsValid` _bp_player_ref_
      (:`Is Valid`
        (if (`/Game/StudentName/Framework/BP_Pawn.can_spawn_prefab_` _bp_player_ref_)
          (`/Game/StudentName/Framework/BP_Pawn.SpawnBuilding` _bp_player_ref_)
          (else
            (`/Game/StudentName/Framework/BP_Pawn.SelectBuilding` _bp_player_ref_)))))))

(event `InputAction|RemoveBuilding` :consume false
  (params (Key :type "Key Structure"))
  (bind _bp_player_ref_ (`self.bp_player_ref_`))
  ;[1 1 1] Game inputs to Player and HUD.
  (:`Pressed`
    (`/Engine/EditorBlueprintResources/StandardMacros.IsValid` _bp_player_ref_
      (:`Is Valid`
        (`/Game/StudentName/Framework/BP_Pawn.RemoveBuilding` _bp_player_ref_)))))

(event `InputAxis|VerticalMovement` :consume false
  (params (AxisValue :type "Float (single-precision)"))
  (bind _bp_player_ref_ (`self.bp_player_ref_`))
  ;[1 1 1] Game inputs to Player and HUD.
  (`/Engine/EditorBlueprintResources/StandardMacros.IsValid` _bp_player_ref_
    (:`Is Valid`
      (`/Game/StudentName/Framework/BP_Pawn.VerticalMovement` _bp_player_ref_ AxisValue))))

(event `InputAxis|TurnCamera` :consume false
  (params (AxisValue :type "Float (single-precision)"))
  (bind _bp_player_ref_ (`self.bp_player_ref_`))
  ;[1 1 1] Game inputs to Player and HUD.
  (`/Engine/EditorBlueprintResources/StandardMacros.IsValid` _bp_player_ref_
    (:`Is Valid`
      (`/Game/StudentName/Framework/BP_Pawn.TurnCamera` _bp_player_ref_ AxisValue))))

(event `InputAxis|Zoom` :consume false
  (params (AxisValue :type "Float (single-precision)"))
  (bind _bp_player_ref_ (`self.bp_player_ref_`))
  ;[1 1 1] Game inputs to Player and HUD.
  (`/Engine/EditorBlueprintResources/StandardMacros.IsValid` _bp_player_ref_
    (:`Is Valid`
      (`/Game/StudentName/Framework/BP_Pawn.Zoom` _bp_player_ref_ AxisValue))))

(event `InputAction|ClearAction` :consume false
  (params (Key :type "Key Structure"))
  (bind _bp_player_ref_ (`self.bp_player_ref_`))
  ;[1 1 1] Game inputs to Player and HUD.
  (:`Pressed`
    (`/Engine/EditorBlueprintResources/StandardMacros.IsValid` _bp_player_ref_
      (:`Is Valid`
        (if (`/Game/StudentName/Framework/BP_Pawn.can_spawn_prefab_` _bp_player_ref_)
          (`/Game/StudentName/Framework/BP_Pawn.ClearBuildingToolSelection` _bp_player_ref_)
          (else
            (`/Game/StudentName/Framework/BP_Pawn.ShowElementInfo` _bp_player_ref_)))))))

(event `InputAction|TechonologyTree` :consume false
  (params (Key :type "Key Structure"))
  (bind _bp_hud_ref_ (`self.bp_hud_ref_`))
  ;[1 1 1] Game inputs to Player and HUD.
  (:`Pressed`
    (`/Engine/EditorBlueprintResources/StandardMacros.IsValid` _bp_hud_ref_
      (:`Is Valid`
        (`/Game/StudentName/Framework/BP_HUD.ChangeTechTreeVisibility` _bp_hud_ref_)))))

(event `InputAxis|LateralMovement` :consume false
  (params (AxisValue :type "Float (single-precision)"))
  (bind _bp_player_ref_ (`self.bp_player_ref_`))
  ;[1 1 1] Game inputs to Player and HUD.
  (`/Engine/EditorBlueprintResources/StandardMacros.IsValid` _bp_player_ref_
    (:`Is Valid`
      (`/Game/StudentName/Framework/BP_Pawn.LateralMovement` _bp_player_ref_ AxisValue))))

(event `InputAxis|TurnBuilding`
  (params (AxisValue :type "Float (single-precision)"))
  (bind _bp_player_ref_ (`self.bp_player_ref_`))
  ;[1 1 1] Game inputs to Player and HUD.
  (`/Engine/EditorBlueprintResources/StandardMacros.IsValid` _bp_player_ref_
    (:`Is Valid`
      (`/Game/StudentName/Framework/BP_Pawn.TurnBuilding` _bp_player_ref_ AxisValue))))

(event `self.ReceiveTick`
  (params (DeltaSeconds :type "Float (single-precision)")))

(fn `UserConstructionScript`)