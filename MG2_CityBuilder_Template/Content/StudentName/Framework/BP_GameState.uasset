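; Game state for a city-builder, holding resources, money, population, age, techs and the game calendar.
; A looping timer advances months and years, and most changes are pushed through BP_GameInstance calls to broadcast updates.
; Helper functions check and deduct building costs, query tech and unique-building status, and strip excess workers from buildings when population drops.
; UpdateResource crosses Iron and Gold, so each type modifies the other's variable.
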(event `self.ReceiveBeginPlay`
  ;[1 1 1] Precatching zone.
  (bind _asbp_game_instance (cast `/Game/StudentName/Framework/BP_GameInstance` (`GameplayStatics.GetGameInstance`)))
  (set `self.game_instance_ref_` _asbp_game_instance)
  ;[1 1 1] This piece of code adds a new month each "X" seconds, and adds new year per twelve months.
  (`KismetSystemLibrary.K2_SetTimerDelegate` (delegate `CustomEvent_0`) (`self.game_speed_`) true))

(event `CustomEvent_0`
  ;[1 1 1] This piece of code adds a new month each "X" seconds, and adds new year per twelve months.
  (bind _result (`/Engine/EditorBlueprintResources/StandardMacros.IncrementInt` (`self.month_`))
    (:`  `
      (if (== (/ _result 12) 1)
        (set `self.month_` 0)
        (`/Engine/EditorBlueprintResources/StandardMacros.IncrementInt` (`self.year_`)
          (:`  `
            (`/Game/StudentName/Framework/BP_GameInstance.UpdateDate` (`self.game_instance_ref_`) (`self.month_`) (`self.year_`))))
        (else
          (`/Game/StudentName/Framework/BP_GameInstance.UpdateDate` (`self.game_instance_ref_`) (`self.month_`) (`self.year_`)))))))

(fn `CheckIfBuildingTechIsDiscovered`
  (params (BuildingType :type "/Game/StudentName/Placeables/Buildings/EBuildingType Enum" :default "NewEnumerator2"))
  (returns (IsDiscovered :type Boolean))
  (bind (_techs__towncenter _techs__house _techs__storage _techs__lumbercamp _techs__sawmill _techs__goldminery _techs__ironminery) (break `/Game/StudentName/UI/TechnologyTree/TechTreeTasks/S_TechCollection` (`self.techs_`)))
  ;[1 1 1] TODO designer: each "EBuildingType" should be allowed in this "Select". Update this select when updating "EBuildingType" enum.
  (return (select `/Game/StudentName/Placeables/Buildings/EBuildingType` BuildingType :`NewEnumerator2` true :`NewEnumerator6` _techs__towncenter :`NewEnumerator0` _techs__house :`NewEnumerator7` _techs__storage :`NewEnumerator1` _techs__lumbercamp :`NewEnumerator3` _techs__sawmill :`NewEnumerator5` _techs__goldminery :`NewEnumerator4` _techs__ironminery)))

(fn `CheckIfIsUniqueBuilding`
  (params (type :type "/Game/StudentName/Placeables/Buildings/EBuildingType Enum" :default "NewEnumerator2"))
  (returns (is_unique_building :type Boolean))
  ;[1 1 1] TODO designer: each "EBuildingType" should be allowed in this "Select". Update this select when updating "EBuildingType" enum.
  (return (select `/Game/StudentName/Placeables/Buildings/EBuildingType` type :`NewEnumerator6` true)))

(fn `CheckIfResourcesAndAgeAreAvailable`
  (params (data_cost :type "/Game/StudentName/Placeables/Buildings/S_ElementCost Structure"))
  (returns (can_spawn :type Boolean))
  (bind (_neededwood _neededgold _needediron _neededage _neededmoney) (break `/Game/StudentName/Placeables/Buildings/S_ElementCost` data_cost))
  ;[1 1 1] This is a method called in "SpawnBuilding" method from "BP_Pawn" class and only checks if we can build a new resource.
  (return (and (<= (`.Cost_6_3868A9FA4671EC9D83A99786C696951E` (break `/Game/StudentName/Placeables/Buildings/S_ResourceQuantity` _neededwood)) (`self.wood_`)) (<= (`.Cost_6_3868A9FA4671EC9D83A99786C696951E` (break `/Game/StudentName/Placeables/Buildings/S_ResourceQuantity` _neededgold)) (`self.gold_`)) (<= (`.Cost_6_3868A9FA4671EC9D83A99786C696951E` (break `/Game/StudentName/Placeables/Buildings/S_ResourceQuantity` _needediron)) (`self.iron_`)) (<= _neededage (`self.age_`)) (<= _neededmoney (`self.money_`)))))

(fn `CheckIfUniqueBuildingIsBuilt`
  (params (type :type "/Game/StudentName/Placeables/Buildings/EBuildingType Enum" :default "NewEnumerator2"))
  (returns (is_built :type Boolean))
  ;[1 1 1] TODO designer: update this select when updating building types and unique building flags.
  (return (select `/Game/StudentName/Placeables/Buildings/EBuildingType` type :`NewEnumerator6` (`.TownCenter_2_732A41A34AEC6ADDF3B99DB0C0740C10` (break `/Game/StudentName/Placeables/Buildings/S_UniqueBuilding` (`self.unique_buildings_state_`))))))

(fn `CheckIfWorkersExceedsPopulation`
  (locals (diff_population :type Integer))
  (if (> (`self.active_population_`) (`self.population_`))
    (set `local.diff_population` (- (`self.active_population_`) (`self.population_`)))
    (bind _outactors (`GameplayStatics.GetAllActorsOfClass` "/Game/StudentName/Placeables/Buildings/BP_BasicBuilding.BP_BasicBuilding_C"))
    (for _array_element _outactors
      (if (> (`local.diff_population`) (`/Game/StudentName/Placeables/Buildings/BP_BasicBuilding.building_workers_` _array_element))
        (bind _output_get (set `local.diff_population` (- (`local.diff_population`) (`/Game/StudentName/Placeables/Buildings/BP_BasicBuilding.building_workers_` _array_element))))
        (set `/Game/StudentName/Placeables/Buildings/BP_BasicBuilding.building_workers_` 0 _array_element)
        (else
          (set `/Game/StudentName/Placeables/Buildings/BP_BasicBuilding.building_workers_` (- (`/Game/StudentName/Placeables/Buildings/BP_BasicBuilding.building_workers_` _array_element) (`local.diff_population`)) _array_element)
          (set `local.diff_population` 0)))
      (`/Game/StudentName/Placeables/Buildings/BP_BasicBuilding.UpdateWorkerMultiplier` _array_element)
      (if (<= _output_get 0)
        (break)))
    (set `self.active_population_` (`self.population_`))
    (return)
    (else
      (return))))

(fn `UpdateAge`
  (params (new_age :type "/Game/StudentName/Placeables/EAgeState Enum" :default "NewEnumerator3"))
  ;[1 1 1] TODO designer: enable some sound in this point?
  (bind _output_get (set `self.age_` new_age))
  (`/Game/StudentName/Framework/BP_GameInstance.UpdateAge` (`self.game_instance_ref_`) _output_get)
  (return))

(fn `UpdatePopulation`
  (params (increment_population_ :type Integer))
  ;[1 1 1] This method is used to update village population when a new building is built.
  (set `self.population_` (+ increment_population_ (`self.population_`)))
  (return))

(fn `UpdatePopulationAndInfo`
  (params (increment_population :type Integer))
  (bind _game_instance_ref_ (`self.game_instance_ref_`))
  ;[1 1 1] This method is used to update village population when a new building is built.
  (bind _output_get (set `self.population_` (+ increment_population (`self.population_`))))
  (`/Engine/EditorBlueprintResources/StandardMacros.IsValid` _game_instance_ref_
    (:`Is Valid`
      (`/Game/StudentName/Framework/BP_GameInstance.UpdatePopulation` _game_instance_ref_ (`self.active_population_`) _output_get)
      (return))
    (:`Is Not Valid`
      (return))))

(fn `UpdateResource`
  (params (type :type "/Game/StudentName/Placeables/Resources/EResourceType Enum" :default "NewEnumerator0") (quantity :type "Float (double-precision)"))
  (bind _returnvalue (+ (select `/Game/StudentName/Placeables/Resources/EResourceType` type :`NewEnumerator0` (`self.wood_`) :`NewEnumerator1` (`self.gold_`) :`NewEnumerator2` (`self.iron_`)) quantity))
  ;[1 1 1] TODO designer: change resources name and add or delete as resources as needed. Operation can be done in positive or negative, just use the correct value in the function call.
  (switch `/Game/StudentName/Placeables/Resources/EResourceType` type
    (:`NewEnumerator0`
      (bind _output_get (set `self.wood_` _returnvalue))
      (if (< _output_get 0.0)
        (set `self.wood_` 0.0)))
    (:`NewEnumerator1`
      (bind _output_get_2 (set `self.gold_` _returnvalue))
      (if (< _output_get_2 0.0)
        (set `self.gold_` 0.0)))
    (:`NewEnumerator2`
      (bind _output_get_3 (set `self.iron_` _returnvalue))
      (if (< _output_get_3 0.0)
        (set `self.iron_` 0.0))))
  (`/Game/StudentName/Framework/BP_GameInstance.UpdateResourcesInfo` (`self.game_instance_ref_`))
  (return))

(fn `UpdateResourcesWhenPurchasing`
  (params (Cost :type "/Game/StudentName/Placeables/Buildings/S_ElementCost Structure"))
  (bind (_neededwood _neededgold _needediron _neededage _neededmoney) (break `/Game/StudentName/Placeables/Buildings/S_ElementCost` Cost))
  ;[1 1 1] TODO designer: update this piece of Blueprint with the operations related with the new attributes that you will create for your game.
  (`|ExecutionSequence`
    (:`then_0`
      (set `self.wood_` (- (`self.wood_`) (`.Cost_6_3868A9FA4671EC9D83A99786C696951E` (break `/Game/StudentName/Placeables/Buildings/S_ResourceQuantity` _neededwood))))
      (set `self.gold_` (- (`self.gold_`) (`.Cost_6_3868A9FA4671EC9D83A99786C696951E` (break `/Game/StudentName/Placeables/Buildings/S_ResourceQuantity` _neededgold)))))
    (:`then_1`
      (set `self.iron_` (- (`self.iron_`) (`.Cost_6_3868A9FA4671EC9D83A99786C696951E` (break `/Game/StudentName/Placeables/Buildings/S_ResourceQuantity` _needediron)))))
    (:`then_2`
      (set `self.money_` (- (`self.money_`) _neededmoney)))
    (:`then_3`
      ;[1 1 1] Finally, updates resources!!
      (`/Game/StudentName/Framework/BP_GameInstance.UpdateResourcesInfo` (`self.game_instance_ref_`))
      (return))))

(fn `UserConstructionScript`)